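; HUD for the cat game that owns the in-game UI and the pause menu.
; On BeginPlay it casts the player to the cat character, shows the in-game widget and pre-creates the pause menu with references to itself and the cat.
; Custom events open and close the menu, toggling pause, cursor and input mode.
; Game over reuses the pause menu widget, switched to its GameOver page.
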(event `self.ReceiveBeginPlay`
  (bind _asbp_third_person_character_cat (cast `/Game/00_MyContent/Blueprints/CharacterBlueprint/BP_ThirdPersonCharacter_Cat` (`GameplayStatics.GetPlayerCharacter` 0)))
  (bind _output_get (set `self.Player` _asbp_third_person_character_cat))
  (`|ExecutionSequence`
    (:`then_0`
      ;[1 1 1] In Game UI
      (bind _returnvalue (`|CreateWidget` "/Game/00_MyContent/Blueprints/Widget/WBP_CatGame.WBP_CatGame_C" null _output_get))
      (bind _output_get_2 (set `self.InGame Widget` _returnvalue))
      (`UserWidget.AddToPlayerScreen` _output_get_2 0))
    (:`then_1`
      ;[1 1 1] Pause Menu
      (bind _returnvalue_2 (`|CreateWidget` "/Game/00_MyContent/Blueprints/Widget/WBP_PauseMenu.WBP_PauseMenu_C" null self _output_get))
      (set `self.PauseMenu Widget` _returnvalue_2))))

(event `PauseMenu_Open`
  (bind _returnvalue (`GameplayStatics.GetPlayerController` 0))
  (bind _pausemenu_widget (`self.PauseMenu Widget`))
  ;[1 0.1875 0.1875] PauseMenu Custom Events
  (`GameplayStatics.SetGamePaused` true)
  (`UserWidget.AddToViewport` _pausemenu_widget 0)
  (set `UserWidget.bIsFocusable` true _pausemenu_widget)
  (set `PlayerController.bShowMouseCursor` true _returnvalue)
  (`WidgetBlueprintLibrary.SetInputMode_UIOnlyEx` _returnvalue (`self.PauseMenu Widget`)))

(event `PauseMenuClose`
  ;[1 0.1875 0.1875] PauseMenu Custom Events
  (`GameplayStatics.SetGamePaused` false)
  (set `PlayerController.bShowMouseCursor` false (`GameplayStatics.GetPlayerController` 0))
  (`Widget.RemoveFromParent` (`self.PauseMenu Widget`))
  (`WidgetBlueprintLibrary.SetInputMode_GameOnly` (`GameplayStatics.GetPlayerController` 0)))

(event `GameOverEvent`
  (bind _pausemenu_widget (`self.PauseMenu Widget`))
  ;[1 1 1] GameOverScreen
  (`GameplayStatics.SetGamePaused` true)
  (`UserWidget.AddToViewport` (`self.PauseMenu Widget`) 0)
  (bind _output_get (set `/Game/00_MyContent/Blueprints/Widget/WBP_PauseMenu.PauseMenu_Enumerator` "NewEnumerator3" _pausemenu_widget))
  (`WidgetSwitcher.SetActiveWidgetIndex` (`/Game/00_MyContent/Blueprints/Widget/WBP_PauseMenu.WidgetSwitcher` _pausemenu_widget) (select `/Game/00_MyContent/Blueprints/Widget/Enum_PauseTabs` _output_get :`NewEnumerator1` 2 :`NewEnumerator2` 1 :`NewEnumerator3` 3))
  (set `PlayerController.bShowMouseCursor` true (`GameplayStatics.GetPlayerController` 0))
  (`WidgetBlueprintLibrary.SetInputMode_UIOnlyEx` (`GameplayStatics.GetPlayerController` 0) (`self.PauseMenu Widget`)))

(fn `UserConstructionScript`)