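; BP_CatFood is a one-time food pickup for the player's cat character.
; Its Interaction event sets a Used guard, casts the player pawn to BP_ThirdPersonCharacter_Cat and triggers its Eating event.
; It then hides the food bag mesh, activates a Niagara disappearance effect and destroys itself after a delay.
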(event `/Game/00_MyContent/Blueprints/BP_Interface/BP_Interface_Interaction.Interaction`
  ;[1 1 1] Interaction with Cat
  (if (not (`self.Used`))
    (set `self.Used` true)
    (bind _asbp_third_person_character_cat (cast `/Game/00_MyContent/Blueprints/CharacterBlueprint/BP_ThirdPersonCharacter_Cat` (`GameplayStatics.GetPlayerPawn` 0)))
    (`/Game/00_MyContent/Blueprints/CharacterBlueprint/BP_ThirdPersonCharacter_Cat.Eating` _asbp_third_person_character_cat)
    (`SceneComponent.SetVisibility` (`self.cat_food_bag`) false false)
    (`ActorComponent.Activate` (`self.NS_Food_Disappearance`) false)
    (`KismetSystemLibrary.Delay` 10.0)
    (`self.K2_DestroyActor`)))

(fn `UserConstructionScript`)