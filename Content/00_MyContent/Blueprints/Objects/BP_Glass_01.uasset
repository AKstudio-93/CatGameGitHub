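; BP_Glass_01 is an interactable glass prop that the cat player character breaks to gain evilness.
; The construction script gives it a random mesh and material from arrays.
; The interface Interaction event calls EvilnessAdd on the cat, removes the mesh, plays a glass sound and activates NSGlass, then destroys the actor after a delay.
; The two-sound Select always picks Glass01, because RandomInteger(1) only returns zero.
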(event `/Game/00_MyContent/Blueprints/BP_Interface/BP_Interface_Interaction.Interaction`
  ;[1 1 1] Interaction From Interface Blueprint
  (bind _asbp_third_person_character_cat (cast `/Game/00_MyContent/Blueprints/CharacterBlueprint/BP_ThirdPersonCharacter_Cat` (`GameplayStatics.GetPlayerCharacter` 0)))
  (`/Game/00_MyContent/Blueprints/CharacterBlueprint/BP_ThirdPersonCharacter_Cat.Evilness_add` _asbp_third_person_character_cat)
  (`ActorComponent.K2_DestroyComponent` (`self.SM_Baker_SM_Baker_F`))
  (`GameplayStatics.SpawnSoundAtLocation` (select `int` (`KismetMathLibrary.RandomInteger` 1) :`0` "/Game/00_MyContent/SFX/Glass01.Glass01" :`1` "/Game/00_MyContent/SFX/Glass02.Glass02" :!type "SoundBase Object Reference") (`SceneComponent.K2_GetComponentLocation` (`self.NS_Glass`)) (struct) 1.0 1.0 0.0 null null)
  (`ActorComponent.Activate` (`self.NS_Glass`) false)
  (`KismetSystemLibrary.Delay` 4.0)
  (`self.K2_DestroyActor`))

(fn `UserConstructionScript`
  (bind _target (`self.Target`))
  (bind _materialarray (`self.MaterialArray`))
  ;[1 1 1] Replace with a random mesh in the array
  (`StaticMeshComponent.SetStaticMesh` (`self.SM_Baker_SM_Baker_F`) (`|GetArrayItem` _target (`KismetMathLibrary.RandomIntegerInRange` 0 (- (`KismetArrayLibrary.Array_Length` _target) 1))))
  (`PrimitiveComponent.SetMaterial` (`self.SM_Baker_SM_Baker_F`) 0 (`|GetArrayItem` _materialarray (`KismetMathLibrary.RandomIntegerInRange` 0 (- (`KismetArrayLibrary.Array_Length` _materialarray) 1)))))